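; BP_Enemy_Shrooms_pewpew is a patrolling shooter enemy that damages the player on contact and awards coins on death.
; Tick walks it forward and uses a Delay to fire BP_Enemy_bullet about every second, or destroys it at zero health.
; Wall and edge triggers flip its direction, ignoring the player's forward attack collider for walls.
; AnyDamage applies knockback in a fixed direction; DamageEnemy picks direction from the player's sword collider.
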(event OnComponentBeginOverlap(wall_detect)
  (params (OverlappedComponent :type Primitive%20Component%20Object%20Reference) (OtherActor :type Actor%20Object%20Reference) (OtherComp :type Primitive%20Component%20Object%20Reference) (OtherBodyIndex :type Integer) (bFromSweep :type Boolean) (SweepResult :type Hit%20Result%20Structure%20%28by%20ref%29))
  (bind _asbp_player (Utilities|Casting|CastToBP_Player (Game|Player|GetPlayerPawn 0)))
  (if (!= (Variables|/Game/PaperAssets/Character/BP_Player.BP_Player_C|GetAttackForward _asbp_player) OtherComp)
    (CallFunction|FlipChar)))

(event OnComponentEndOverlap(edge_detect)
  (params (OverlappedComponent :type Primitive%20Component%20Object%20Reference) (OtherActor :type Actor%20Object%20Reference) (OtherComp :type Primitive%20Component%20Object%20Reference) (OtherBodyIndex :type Integer))
  (CallFunction|FlipChar))

(event EventBeginPlay)

(event Collision|EventHit
  (params (MyComp :type Primitive%20Component%20Object%20Reference) (Other :type Actor%20Object%20Reference) (OtherComp :type Primitive%20Component%20Object%20Reference) (bSelfMoved :type Boolean) (HitLocation :type Vector :default "0, 0, 0") (HitNormal :type Vector :default "0, 0, 0") (NormalImpulse :type Vector :default "0, 0, 0") (Hit :type Hit%20Result%20Structure%20%28by%20ref%29))
  (bind _asbp_player (Utilities|Casting|CastToBP_Player Other))
  (Game|Damage|ApplyDamage _asbp_player 1.0 0 self))

(event EventTick
  (params (DeltaSeconds :type Float%20%28single-precision%29))
  (if (<= (Variables|Default|GetHealth) 0.0)
    (Actor|DestroyActor)
    (bind _asbp_player (Utilities|Casting|CastToBP_Player (Game|Player|GetPlayerPawn 0)))
    (Variables|/Game/PaperAssets/Character/UI/UI.UI_C|SetNumCoins (Variables|/Game/PaperAssets/Character/BP_Player.BP_Player_C|GetBaseUI _asbp_player) (+ (Variables|/Game/PaperAssets/Character/UI/UI.UI_C|GetNumCoins (Variables|/Game/PaperAssets/Character/BP_Player.BP_Player_C|GetBaseUI _asbp_player)) 10))
    (else
      (Pawn|Input|AddMovementInput (Transformation|GetActorForwardVector) 1.0 false)
      (Utilities|FlowControl|Delay 1.0)
      (CallFunction|Shoot))))

(event Game|Damage|EventAnyDamage
  (params (Damage :type Float%20%28single-precision%29) (DamageType :type Damage%20Type%20Object%20Reference) (InstigatedBy :type Controller%20Object%20Reference) (DamageCauser :type Actor%20Object%20Reference))
  (Variables|Default|SetBeingDamaged true)
  (Variables|Default|SetHealth (- (Variables|Default|GetHealth) Damage))
  (if true
    (Character|LaunchCharacter "2000.000000,0.000000,50.000000" false false)
    (else
      (Character|LaunchCharacter "-2000.000000,0.000000,50.000000" false false)))
  (Utilities|FlowControl|Delay 0.1)
  (Variables|Default|SetBeingDamaged false))

(event Collision|EventActorBeginOverlap
  (params (OtherActor :type Actor%20Object%20Reference)))

(fn ConstructionScript)

(fn FlipChar
  (Transformation|SetActorRotation (Math|Rotator|CombineRotators (Transformation|GetActorRotation) "0.000000,180.000000,0.000000"))
  (Variables|Default|Setflipped (not (Variables|Default|Getflipped))))

(fn Shoot
  (Game|SpawnActorfromClass "/Game/enemies/BP_Enemy_bullet.BP_Enemy_bullet_C" (Math|Transform|MakeTransform (Transformation|GetActorLocation) "0, 0, 0" "1.000000,1.000000,1.000000") "AlwaysSpawn" "MultiplyWithRoot" self 0))

(fn DamageEnemy
  (params (A :type Object%20Object%20Reference) (B :type Object%20Object%20Reference))
  (bind _asbp_player (Utilities|Casting|CastToBP_Player (Game|Player|GetPlayerPawn 0)))
  (if (and (or (== A (Variables|/Game/PaperAssets/Character/BP_Player.BP_Player_C|GetAttackBack _asbp_player)) (== (Variables|/Game/PaperAssets/Character/BP_Player.BP_Player_C|GetAttackForward _asbp_player) B)) (not (Variables|Default|GetBeingDamaged)))
    (Variables|Default|SetBeingDamaged true)
    (Variables|Default|SetHealth (- (Variables|Default|GetHealth) (Variables|/Game/PaperAssets/Character/BP_Player.BP_Player_C|GetSwordDamage _asbp_player)))
    (if (== (Variables|/Game/PaperAssets/Character/BP_Player.BP_Player_C|GetAttackForward _asbp_player) B)
      (Character|LaunchCharacter "2000.000000,0.000000,50.000000" false false)
      (else
        (Character|LaunchCharacter "-2000.000000,0.000000,50.000000" false false)))))