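; Projectile for the BP_Enemy_Shrooms_pewpew enemy that damages the player on contact.
; The construction script casts its owner to that enemy, adds a projectile movement component and fires along local X, reversed when the owner is Flipped.
; BulletBox overlap deals damage and destroys the bullet only on the player's capsule, ignoring other player components.
; It passes through shooters of that enemy class and is destroyed by any other actor.
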(event OnComponentBeginOverlap(BulletBox)
  (params (OverlappedComponent :type Primitive%20Component%20Object%20Reference) (OtherActor :type Actor%20Object%20Reference) (OtherComp :type Primitive%20Component%20Object%20Reference) (OtherBodyIndex :type Integer) (bFromSweep :type Boolean) (SweepResult :type Hit%20Result%20Structure%20%28by%20ref%29))
  (bind _asbp_player (Utilities|Casting|CastToBP_Player OtherActor)
    (:then
      (if (== (Variables|/Script/Engine.Character|GetCapsuleComponent _asbp_player) OtherComp)
        (Game|Damage|ApplyDamage OtherActor 1.0 0 self)
        (Actor|DestroyActor)))
    (:CastFailed
      (Utilities|Casting|CastToBP_Enemy_Shrooms_pewpew OtherActor
        (:CastFailed
          (Actor|DestroyActor))))))

(event EventBeginPlay)

(event Collision|EventActorBeginOverlap
  (params (OtherActor :type Actor%20Object%20Reference)))

(event EventTick
  (params (DeltaSeconds :type Float%20%28single-precision%29)))

(fn ConstructionScript
  (bind _asbp_enemy_shrooms_pewpew (Utilities|Casting|CastToBP_Enemy_Shrooms_pewpew (Components|GetOwner)))
  (bind _returnvalue (AddComponent|AddProjectileMovementComponent))
  (if (Variables|/Game/enemies/BP_Enemy_Shrooms_pewpew.BP_Enemy_Shrooms_pewpew_C|Getflipped _asbp_enemy_shrooms_pewpew)
    (Game|Components|ProjectileMovement|SetVelocityinLocalSpace _returnvalue (Math|Vector|MakeVector -7.5e+02 0.0 0.0))
    (else
      (Game|Components|ProjectileMovement|SetVelocityinLocalSpace _returnvalue (Math|Vector|MakeVector 7.5e+02 0.0 0.0)))))