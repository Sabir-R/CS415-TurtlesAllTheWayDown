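; Slime enemy for a side-view game that hops toward the player on the X axis when within range, flipping to face them.
; Tick uses a Delay to pace SlimeMovement launches, and destroys the slime at zero health, adding coins to the player's UI counter.
; Hitting the player deals damage and destroys the slime.
; Damage taken lowers Health and applies knockback, always toward +X because its direction branch is fixed true.
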(event EventBeginPlay)

(event Collision|EventHit
  (params (MyComp :type Primitive%20Component%20Object%20Reference) (Other :type Actor%20Object%20Reference) (OtherComp :type Primitive%20Component%20Object%20Reference) (bSelfMoved :type Boolean) (HitLocation :type Vector :default "0, 0, 0") (HitNormal :type Vector :default "0, 0, 0") (NormalImpulse :type Vector :default "0, 0, 0") (Hit :type Hit%20Result%20Structure%20%28by%20ref%29))
  (bind _asbp_player (Utilities|Casting|CastToBP_Player Other))
  (Game|Damage|ApplyDamage _asbp_player 1.0 0 self)
  (Actor|DestroyActor))

(event EventTick
  (params (DeltaSeconds :type Float%20%28single-precision%29))
  (if (<= (Variables|Default|GetHealth) 0.0)
    (Actor|DestroyActor)
    (bind _asbp_player (Utilities|Casting|CastToBP_Player (Game|Player|GetPlayerPawn 0)))
    (Variables|/Game/PaperAssets/Character/UI/UI.UI_C|SetNumCoins (Variables|/Game/PaperAssets/Character/BP_Player.BP_Player_C|GetBaseUI _asbp_player) (+ (Variables|/Game/PaperAssets/Character/UI/UI.UI_C|GetNumCoins (Variables|/Game/PaperAssets/Character/BP_Player.BP_Player_C|GetBaseUI _asbp_player)) 10))
    (else
      (Utilities|FlowControl|Delay 2.0)
      (CallFunction|SlimeMovement))))

(event Game|Damage|EventAnyDamage
  (params (Damage :type Float%20%28single-precision%29) (DamageType :type Damage%20Type%20Object%20Reference) (InstigatedBy :type Controller%20Object%20Reference) (DamageCauser :type Actor%20Object%20Reference))
  (Variables|Default|SetBeingDamaged true)
  (Variables|Default|SetHealth (- (Variables|Default|GetHealth) Damage))
  (if true
    (Character|LaunchCharacter "2000.000000,0.000000,50.000000" false false)
    (else
      (Character|LaunchCharacter "-2000.000000,0.000000,50.000000" false false)))
  (Utilities|FlowControl|Delay 0.1)
  (Variables|Default|SetBeingDamaged false))

(fn ConstructionScript)

(fn SlimeMovement
  (bind _returnvalue (Transformation|GetActorLocation))
  (bind _returnvalue_2 (Game|GetPlayerCharacter 0))
  (bind _returnvalue_3 (Transformation|GetActorLocation _returnvalue_2))
  (bind _returnvalue_4 (- (.x _returnvalue) (.x _returnvalue_3)))
  (bind _returnvalue_5 (Math|Float|Sign(Float) _returnvalue_4))
  (if (< (Math|Vector|Distance2D(Vector) (Math|Vector|MakeVector (.x _returnvalue) 0.0 (.z _returnvalue)) (Math|Vector|MakeVector (.x _returnvalue_3) 0.0 (.z _returnvalue_3))) 1.5e+03)
    (Character|LaunchCharacter (Math|Vector|MakeVector (* _returnvalue_5 -3e+02) 0.0 3e+02) true true)
    (if (Class|KismetMathLibrary|XORBoolean (> _returnvalue_5 0.0) (Variables|Default|Getflipped))
      (CallFunction|FlipChar))))

(fn FlipChar
  (Transformation|SetActorRotation (Math|Rotator|CombineRotators (Transformation|GetActorRotation) "0.000000,180.000000,0.000000"))
  (Variables|Default|Setflipped (not (Variables|Default|Getflipped))))