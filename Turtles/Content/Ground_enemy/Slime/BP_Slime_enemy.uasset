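; Slime ground enemy that hands the player to its AI controller through an Aggro overlap gated by DoOnce.
; Hitting the player applies damage, then calls BounceToward with a zero direction; the event itself just adds forced movement input.
; Any damage launches the slime along X away from the damage causer, then destroys it after a short delay.
; HealthCheck and the construction script are empty.
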(event OnComponentBeginOverlap(Aggro)
  (params (OverlappedComponent :type Primitive%20Component%20Object%20Reference) (OtherActor :type Actor%20Object%20Reference) (OtherComp :type Primitive%20Component%20Object%20Reference) (OtherBodyIndex :type Integer) (bFromSweep :type Boolean) (SweepResult :type Hit%20Result%20Structure%20%28by%20ref%29))
  (bind _asbp_player (Utilities|Casting|CastToBP_Player OtherActor))
  (Utilities|FlowControl|DoOnce false
    (:Completed
      (bind _asaic__slime (Utilities|Casting|CastToAIC__Slime (AI|GetAIController self)))
      (Default|SetTargetPLayer _asaic__slime _asbp_player))))

(event Custom|BounceToward
  (params (WorldDirection :type Vector) (ScaleValue :type Float%20%28single-precision%29))
  (Pawn|Input|AddMovementInput WorldDirection ScaleValue true))

(event Collision|EventHit
  (params (MyComp :type Primitive%20Component%20Object%20Reference) (Other :type Actor%20Object%20Reference) (OtherComp :type Primitive%20Component%20Object%20Reference) (bSelfMoved :type Boolean) (HitLocation :type Vector :default "0, 0, 0") (HitNormal :type Vector :default "0, 0, 0") (NormalImpulse :type Vector :default "0, 0, 0") (Hit :type Hit%20Result%20Structure%20%28by%20ref%29))
  ;[1 1 1] Flying Attack
  (bind _asbp_player (Utilities|Casting|CastToBP_Player Other))
  (Game|Damage|ApplyDamage _asbp_player 1.0 0 self)
  (CallFunction|BounceToward "0, 0, 0" 1.0))

(event Game|Damage|EventAnyDamage
  (params (Damage :type Float%20%28single-precision%29) (DamageType :type Damage%20Type%20Object%20Reference) (InstigatedBy :type Controller%20Object%20Reference) (DamageCauser :type Actor%20Object%20Reference))
  ;[1 1 1] Flying enemy Health
  (if (> (- (.x (Transformation|GetActorLocation DamageCauser)) (.x (Transformation|GetActorLocation self))) 0.0)
    (Character|LaunchCharacter "-1500.000000,0.000000,150.000000" false false)
    (else
      (Character|LaunchCharacter "1500.000000,0.000000,150.000000" false false)))
  (Utilities|FlowControl|Delay 0.1)
  (Actor|DestroyActor))

(fn ConstructionScript)

(fn HealthCheck)