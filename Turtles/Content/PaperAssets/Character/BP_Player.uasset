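; Paper2D player character for a side-scrolling platformer, with run, jump and attack driven by Enhanced Input.
; Move input runs along world X and sets a facing value that mirrors the sprite through its X scale.
; Attack raises a flag for a short delay, while a canceled jump zeroes vertical velocity.
; Each tick picks the flipbook from attack, ground and velocity state, shrinking sprite scale for the attack flipbook.
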(event Input|EnhancedActionEvents|EnhancedInputActionIA_Jump
  (params (ActionValue :type Boolean) (ElapsedSeconds :type Float%20%28double-precision%29) (TriggeredSeconds :type Float%20%28double-precision%29) (InputAction :type Input%20Action%20Object%20Reference :default "/Game/PaperAssets/Character/Input/IA_Jump.IA_Jump"))
  (bind _charactermovement (Variables|Character|GetCharacterMovement))
  (:Started
    (Character|Jump))
  (:Canceled
    (Variables|/Script/Engine.MovementComponent|SetVelocity _charactermovement (Math|Vector|MakeVector (.x (Variables|/Script/Engine.MovementComponent|GetVelocity _charactermovement)) (.y (Variables|/Script/Engine.MovementComponent|GetVelocity _charactermovement)) 0.0))
    (Character|StopJumping :!label _label))
  (:Completed
    (goto _label)))

(event Input|EnhancedActionEvents|EnhancedInputActionIA_Move
  (params (ActionValue :type Float%20%28double-precision%29) (ElapsedSeconds :type Float%20%28double-precision%29) (TriggeredSeconds :type Float%20%28double-precision%29) (InputAction :type Input%20Action%20Object%20Reference :default "/Game/PaperAssets/Character/Input/IA_Move.IA_Move"))
  (if (> ActionValue 0.0)
    (Variables|Default|SetForward 1.0)
    (else
      (Variables|Default|SetForward -1.0)))
  (Pawn|Input|AddMovementInput "1.000000,0.000000,0.000000" ActionValue false))

(event Input|EnhancedActionEvents|EnhancedInputActionIA_Attack
  (params (ActionValue :type Boolean) (ElapsedSeconds :type Float%20%28double-precision%29) (TriggeredSeconds :type Float%20%28double-precision%29) (InputAction :type Input%20Action%20Object%20Reference :default "/Game/PaperAssets/Character/Input/IA_Attack.IA_Attack"))
  (Variables|Default|SetIsAttacking true)
  (Utilities|FlowControl|Delay 0.5)
  (Variables|Default|SetIsAttacking false))

(event EventBeginPlay
  (bind _asplayer_controller (Utilities|Casting|CastToPlayerController (Pawn|GetController)))
  (Input|AddMappingContext (PlayerController|LocalPlayerSubsystems|GetEnhancedInputLocalPlayerSubsystem _asplayer_controller) "/Game/PaperAssets/Character/Input/IMC_Platforming.IMC_Platforming" 0 "(bIgnoreAllPressedKeysUntilRelease=True,bForceImmediately=False,bNotifyUserSettings=False)"))

(event Collision|EventActorBeginOverlap
  (params (OtherActor :type Actor%20Object%20Reference)))

(event EventTick
  (params (DeltaSeconds :type Float%20%28single-precision%29))
  (CallFunction|UpdateAnimation))

(fn ConstructionScript)

(fn UpdateAnimation
  (bind _sprite (Variables|Default|GetSprite))
  (if (Variables|Default|GetIsAttacking)
    (Transformation|SetWorldScale3D _sprite (Math|Vector|MakeVector (* (Variables|Default|GetForward) 0.1) 1.0 0.1))
    (Sprite|SetFlipbook _sprite (Variables|Default|GetAttackFlip))
    (else
      (Transformation|SetWorldScale3D (Variables|Default|GetSprite) (Math|Vector|MakeVector (Variables|Default|GetForward) 1.0 1.0))
      (if (AI|Components|NavMovement|IsMovingonGround (Variables|Character|GetCharacterMovement))
        (if (> (Math|Vector|VectorLength (Transformation|GetVelocity)) 0.0)
          (Sprite|SetFlipbook (Variables|Default|GetSprite) "/Game/PaperAssets/Character/FB_Player_run.FB_Player_run")
          (else
            (Sprite|SetFlipbook (Variables|Default|GetSprite) "/Game/PaperAssets/Character/FP_Player_Idle.FP_Player_Idle")))
        (elif (> 0.0 (.z (Transformation|GetVelocity)))
          (Sprite|SetFlipbook (Variables|Default|GetSprite) "/Game/PaperAssets/Character/FP_Player_Fall.FP_Player_Fall")
          (else
            (Sprite|SetFlipbook (Variables|Default|GetSprite) "/Game/PaperAssets/Character/FP_Player_Jump.FP_Player_Jump")))))))