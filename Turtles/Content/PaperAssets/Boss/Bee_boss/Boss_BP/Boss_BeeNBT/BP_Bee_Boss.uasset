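; Paper2D bee boss that chases the player, deals contact damage and shows a health bar.
; Damage knocks it back and calls SetSkyattack, which resumes the recursive AIMoveTo chase or, at exactly 30 health, starts SkyPatrol.
; SkyPatrol flies between fixed points, spawns minion waves on both sides and toggles IsSkyAttack for hive projectiles, then resumes chasing.
; Tick updates the health widget and, at zero health, destroys the boss, shows congratulations and quits.
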(event OnComponentBeginOverlap(Boss_Collision)
  (params (OverlappedComponent :type Primitive%20Component%20Object%20Reference) (OtherActor :type Actor%20Object%20Reference) (OtherComp :type Primitive%20Component%20Object%20Reference) (OtherBodyIndex :type Integer) (bFromSweep :type Boolean) (SweepResult :type Hit%20Result%20Structure%20%28by%20ref%29))
  (Development|PrintString "Collided")
  (bind _asbp_player (Utilities|Casting|CastToBP_Player (Game|Player|GetPlayerPawn 0)))
  (if (== (Variables|/Script/Engine.Character|GetCapsuleComponent _asbp_player) OtherComp)
    (Game|Damage|ApplyDamage (Game|GetPlayerCharacter 0) 1.0 0 self)
    (Development|PrintString (Utilities|String|ToString(Integer) (Variables|/Game/PaperAssets/Character/BP_Player.BP_Player_C|GetHealth _asbp_player)))))

(event Custom|SetSkyattack
  ;[1 1 1] Skyuattack setter
  (if (== (Variables|Default|GetBee_Boss_Health) 3e+01)
    (Variables|Default|SetIsSkyAttack true)
    (CallFunction|SkyPatrol)
    (else
      (CallFunction|Chase))))

(event Custom|SpawnMinionsRight
  ;[1 1 1] Minion Spawn
  (Utilities|FlowControl|Delay 1.0)
  (for _index (range 0 2)
    (AI|SpawnAIFromClass "/Game/PaperAssets/Boss/Bee_boss/Boss_BP/Boss_BeeNBT/BP_Bee_Minons.BP_Bee_Minons_C" 0 "140.000000,60.000000,-600.000000" "0.000000,0.000000,0.000000" false 0)))

(event Custom|Chase
  ;[1 1 1] Phase1 Chase Player from Health is 50,30,10
  (AI|AIMoveTo self "0, 0, 0" (Game|GetPlayerCharacter 0) 5.0 false
    (:then
      (Utilities|FlowControl|Delay 1.0)
      (CallFunction|Chase))
    (:OnSuccess
      (Utilities|FlowControl|Delay 0.2)
      (Sprite|SetFlipbook (Variables|Default|GetSprite) "/Game/PaperAssets/Boss/Bee_boss/FlipBook/FB_Boss_Attack.FB_Boss_Attack")
      (Sprite|SetFlipbook (Variables|Default|GetSprite) "/Game/PaperAssets/Boss/Bee_boss/FlipBook/FB_Boss_Fly.FB_Boss_Fly")
      (CallFunction|Chase))))

(event Custom|SkyPatrol
  ;[1 1 1] Phase 2 Attack player from the sky where the Bee hives shoot projectile. Set IsSkyAttack = true enabling the shoot for the projectiles.(15 second timer)
  (CallFunction|SpawnMinionsRight)
  (Components|MoveComponentTo (Variables|Default|GetCapsuleComponent) "2200.000000,60.000000,-100.000000" "0, 0, 0" false false 0.2 false)
  (Utilities|FlowControl|Delay 5.0)
  (CallFunction|SpawnMinionLeft)
  (Variables|Default|SetIsSkyAttack false)
  (Components|MoveComponentTo (Variables|Default|GetCapsuleComponent) "240.000000,60.000000,-100.000000" "0, 0, 0" false false 0.2 false)
  (CallFunction|SpawnMinionLeft)
  (CallFunction|SpawnMinionsRight)
  (Utilities|FlowControl|Delay 5.0)
  (Components|MoveComponentTo (Variables|Default|GetCapsuleComponent) "2190.000000,60.000000,-600.000000" "0, 0, 0" false false 0.2 false)
  (CallFunction|Chase))

(event Custom|SpawnMinionLeft
  ;[1 1 1] Minion Spawn
  (Utilities|FlowControl|Delay 1.0)
  (for _index (range 0 2)
    (AI|SpawnAIFromClass "/Game/PaperAssets/Boss/Bee_boss/Boss_BP/Boss_BeeNBT/BP_Bee_Minons.BP_Bee_Minons_C" 0 "2220.000000,60.000000,-600.000000" "0.000000,180.000000,0.000000" false 0)))

(event EventBeginPlay
  ;[1 1 1] Boss UI and game logic
  (Variables|Default|SetBee_Boss_Health (Variables|Default|GetMaxBoss_health))
  (bind _returnvalue (UserInterface|CreateWidget "/Game/PaperAssets/Boss/Bee_boss/Boss_BP/Boss_BeeNBT/UI/WB_Boss_Health.WB_Boss_Health_C"))
  (UserInterface|Viewport|AddtoViewport _returnvalue 0)
  (Variables|Default|SetHealthUI _returnvalue)
  (CallFunction|SetSkyattack))

(event Collision|EventActorBeginOverlap
  (params (OtherActor :type Actor%20Object%20Reference)))

(event EventTick
  (params (DeltaSeconds :type Float%20%28single-precision%29))
  (Progress|SetPercent (Variables|/Game/PaperAssets/Boss/Bee_boss/Boss_BP/Boss_BeeNBT/UI/WB_Boss_Health.WB_Boss_Health_C|GetHealthBar (Variables|Default|GetHealthUI)) (/ (Variables|Default|GetBee_Boss_Health) (Variables|Default|GetMaxBoss_health)))
  (if (== (Variables|Default|GetBee_Boss_Health) 0.0)
    (Actor|DestroyActor)
    (bind _returnvalue (UserInterface|CreateWidget "/Game/PaperAssets/Boss/Bee_boss/Boss_BP/Boss_BeeNBT/UI/WB_Congrats.WB_Congrats_C"))
    (UserInterface|Viewport|AddtoViewport _returnvalue 0)
    (Utilities|FlowControl|Delay 0.5)
    (Game|QuitGame 0 "Quit" false)))

(event Game|Damage|EventAnyDamage
  (params (Damage :type Float%20%28single-precision%29) (DamageType :type Damage%20Type%20Object%20Reference) (InstigatedBy :type Controller%20Object%20Reference) (DamageCauser :type Actor%20Object%20Reference))
  ;[1 1 1] Boss Health
  (if (> (- (.x (Transformation|GetActorLocation DamageCauser)) (.x (Transformation|GetActorLocation self))) 0.0)
    (Character|LaunchCharacter "-2000.000000,0.000000,100.000000" true true)
    (else
      (Character|LaunchCharacter "2000.000000,0.000000,100.000000" true true)))
  (Utilities|FlowControl|Delay 0.1)
  (Sprite|SetFlipbook (Variables|Default|GetSprite) "/Game/PaperAssets/Boss/Bee_boss/FlipBook/FB_Boss_Hit.FB_Boss_Hit")
  (Character|LaunchCharacter "0.000000,0.000000,0.000000" true true)
  (Utilities|FlowControl|Delay 0.3)
  (Sprite|SetFlipbook (Variables|Default|GetSprite) "/Game/PaperAssets/Boss/Bee_boss/FlipBook/FB_Boss_Fly.FB_Boss_Fly")
  (bind _output_get (Variables|Default|SetBee_Boss_Health (- (Variables|Default|GetBee_Boss_Health) Damage)))
  (Development|PrintString (Utilities|String|ToString(Text) (Utilities|Text|ToText(Float) _output_get "HalfToEven")))
  (CallFunction|SetSkyattack))

(fn ConstructionScript)

(fn HealthCheck)