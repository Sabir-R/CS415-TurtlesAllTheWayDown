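; BP_Bee_Minons is a bee boss minion that chases the player and deals contact damage.
; From BeginPlay, a Chase event runs AI MoveTo on the player and re-calls itself shortly after each move completes.
; Overlapping the player's capsule with the Minion_attack component applies damage.
; Any damage taken launches the minion away from the damage causer along X, then destroys it after a brief delay.
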(event OnComponentBeginOverlap(Minion_attack)
  (params (OverlappedComponent :type Primitive%20Component%20Object%20Reference) (OtherActor :type Actor%20Object%20Reference) (OtherComp :type Primitive%20Component%20Object%20Reference) (OtherBodyIndex :type Integer) (bFromSweep :type Boolean) (SweepResult :type Hit%20Result%20Structure%20%28by%20ref%29))
  (bind _asbp_player (Utilities|Casting|CastToBP_Player (Game|Player|GetPlayerPawn 0)))
  (if (== (Variables|/Script/Engine.Character|GetCapsuleComponent _asbp_player) OtherComp)
    (Game|Damage|ApplyDamage (Game|GetPlayerCharacter 0) 1.0 0 self)))

(event Custom|Chase
  ;[1 1 1] Phase1 Chase Player from Health is 50,30,10
  (AI|AIMoveTo self "0, 0, 0" (Game|GetPlayerCharacter 0) 5.0 false
    (:then
      (Utilities|FlowControl|Delay 0.2)
      (CallFunction|Chase))))

(event EventBeginPlay
  ;[1 1 1] Minion Chase
  (CallFunction|Chase))

(event Game|Damage|EventAnyDamage
  (params (Damage :type Float%20%28single-precision%29) (DamageType :type Damage%20Type%20Object%20Reference) (InstigatedBy :type Controller%20Object%20Reference) (DamageCauser :type Actor%20Object%20Reference))
  ;[1 1 1] Boss Health
  (if (> (- (.x (Transformation|GetActorLocation DamageCauser)) (.x (Transformation|GetActorLocation self))) 0.0)
    (Character|LaunchCharacter "-1500.000000,60.000000,150.000000" true true)
    (else
      (Character|LaunchCharacter "1500.000000,60.000000,150.000000" true true)))
  (Utilities|FlowControl|Delay 0.1)
  (Actor|DestroyActor))

(fn ConstructionScript)

(fn HealthCheck)