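; BP_BuzzMinions is a flying Bee boss minion, used in phase 2, that chases the player and deals contact damage.
; Its aggro range hands the player to AIC_BuzzMinions once, and a Chase event moves it, flipping it to face its horizontal direction.
; Capsule overlap with the player's capsule applies damage.
; Any damage received launches it away from the damage causer, then destroys it after a brief delay.
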(event OnComponentBeginOverlap(CapsuleComponent)
  (params (OverlappedComponent :type Primitive%20Component%20Object%20Reference) (OtherActor :type Actor%20Object%20Reference) (OtherComp :type Primitive%20Component%20Object%20Reference) (OtherBodyIndex :type Integer) (bFromSweep :type Boolean) (SweepResult :type Hit%20Result%20Structure%20%28by%20ref%29))
  ;[1 1 1] Flying Attack
  (bind _asbp_player (Utilities|Casting|CastToBP_Player (Game|Player|GetPlayerPawn 0)))
  (if (== (Variables|/Script/Engine.Character|GetCapsuleComponent _asbp_player) OtherComp)
    (Game|Damage|ApplyDamage (Game|GetPlayerCharacter 0) 1.0 0 self)))

(event OnComponentBeginOverlap(AggroRange)
  (params (OverlappedComponent :type Primitive%20Component%20Object%20Reference) (OtherActor :type Actor%20Object%20Reference) (OtherComp :type Primitive%20Component%20Object%20Reference) (OtherBodyIndex :type Integer) (bFromSweep :type Boolean) (SweepResult :type Hit%20Result%20Structure%20%28by%20ref%29))
  (bind _asbp_player (Utilities|Casting|CastToBP_Player OtherActor))
  (Utilities|FlowControl|DoOnce false
    (:Completed
      (bind _asaic_buzz_minions (Utilities|Casting|CastToAIC_BuzzMinions (AI|GetAIController self)))
      (Default|SetTargetPlayer _asaic_buzz_minions _asbp_player))))

(event Custom|Chase
  (params (WorldDirection :type Vector) (ScaleValue :type Float%20%28single-precision%29))
  ;[1 1 1] Phase 2 Minions
  (Pawn|Input|AddMovementInput WorldDirection ScaleValue false)
  (Transformation|SetActorRotation (select (< (.X (Math|Vector|BreakVector WorldDirection)) 0.0) "0.000000,180.000000,0.000000" "0, 0, 0")))

(event Game|Damage|EventAnyDamage
  (params (Damage :type Float%20%28single-precision%29) (DamageType :type Damage%20Type%20Object%20Reference) (InstigatedBy :type Controller%20Object%20Reference) (DamageCauser :type Actor%20Object%20Reference))
  ;[1 1 1] Flying enemy Health
  (if (> (- (.x (Transformation|GetActorLocation DamageCauser)) (.x (Transformation|GetActorLocation self))) 0.0)
    (Character|LaunchCharacter "-1500.000000,60.000000,150.000000" true true)
    (else
      (Character|LaunchCharacter "1500.000000,60.000000,150.000000" true true)))
  (Utilities|FlowControl|Delay 0.1)
  (Actor|DestroyActor))

(fn ConstructionScript)

(fn HealthCheck)