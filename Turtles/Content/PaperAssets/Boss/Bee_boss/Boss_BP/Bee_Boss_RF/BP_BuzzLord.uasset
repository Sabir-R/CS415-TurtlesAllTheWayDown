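; BP_BuzzLord is a flying Paper2D bee boss with its own health bar, contact-damage attack and knockback when hit.
; Entering its aggro range hands the player to AIC_BuzzLord as target, and Chase applies movement and flips facing.
; At exactly 20 health it enters phase 2, spawning BP_BuzzMinions at its location.
; At zero it destroys itself, shows a congrats widget and calls QuitGame after a delay.
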(event OnComponentBeginOverlap(AggroRange)
  (params (OverlappedComponent :type Primitive%20Component%20Object%20Reference) (OtherActor :type Actor%20Object%20Reference) (OtherComp :type Primitive%20Component%20Object%20Reference) (OtherBodyIndex :type Integer) (bFromSweep :type Boolean) (SweepResult :type Hit%20Result%20Structure%20%28by%20ref%29))
  ;[1 1 1] Aggro
  (bind _asbp_player (Utilities|Casting|CastToBP_Player OtherActor))
  (Utilities|FlowControl|DoOnce false
    (:Completed
      (bind _asaic_buzz_lord (Utilities|Casting|CastToAIC_BuzzLord (AI|GetAIController self)))
      (Default|SetTargetPlayerBoss _asaic_buzz_lord _asbp_player))))

(event Custom|SpawnMinions
  ;[1 1 1] Spawns Minions at Boss location
  (for _index (range 0 10)
    (AI|SpawnAIFromClass "/Game/PaperAssets/Boss/Bee_boss/Boss_BP/Bee_Boss_RF/BP_BuzzMinions/BP_BuzzMinions.BP_BuzzMinions_C" 0 (Transformation|GetActorLocation self) "0, 0, 0" false 0)
    (Utilities|FlowControl|Delay 5.0)
    (AI|SpawnAIFromClass "/Game/PaperAssets/Boss/Bee_boss/Boss_BP/Bee_Boss_RF/BP_BuzzMinions/BP_BuzzMinions.BP_BuzzMinions_C" 0 (Transformation|GetActorLocation self) "0, 0, 0" false 0)))

(event Custom|MinionSpawnTrigger
  ;[1 1 1] Phase 2 Minion Spawn Chase
  (if (Variables|Default|GetIsPhase2)
    (Development|PrintString "Phase2")
    (CallFunction|SpawnMinions)
    (else
      (CallFunction|Chase "0, 0, 0" 1.0))))

(event Custom|BossDeath
  ;[1 1 1] Dead
  (if true
    (Actor|DestroyActor)
    (Widget|RemovefromParent (Variables|Default|GetBuzzLordHealthUI))
    (bind _returnvalue (UserInterface|CreateWidget "/Game/PaperAssets/Boss/Bee_boss/Boss_BP/Bee_Boss_RF/UI/WB_Congrats_BuzzLord.WB_Congrats_BuzzLord_C"))
    (UserInterface|Viewport|AddtoViewport _returnvalue 0)
    (Utilities|FlowControl|Delay 0.5)
    (Game|QuitGame 0 "Quit" false)))

(event Custom|Chase
  (params (WorldDirection :type Vector) (ScaleValue :type Float%20%28single-precision%29))
  ;[1 1 1] Phase 1 Chase
  (Pawn|Input|AddMovementInput WorldDirection ScaleValue false)
  (Transformation|SetActorRotation (select (< (.X (Math|Vector|BreakVector WorldDirection)) 0.0) "0.000000,180.000000,0.000000" "0, 0, 0")))

(event EventBeginPlay
  ;[1 1 1] When The Game Starts
  (Variables|Default|SetBuzzLordHealth (Variables|Default|GetMax_BuzzLord_Health))
  (bind _returnvalue (UserInterface|CreateWidget "/Game/PaperAssets/Boss/Bee_boss/Boss_BP/Bee_Boss_RF/UI/WB_BuzzLord_Health.WB_BuzzLord_Health_C"))
  (UserInterface|Viewport|AddtoViewport _returnvalue 0)
  (Variables|Default|SetBuzzLordHealthUI _returnvalue)
  (CallFunction|MinionSpawnTrigger))

(event Collision|EventHit
  (params (MyComp :type Primitive%20Component%20Object%20Reference) (Other :type Actor%20Object%20Reference) (OtherComp :type Primitive%20Component%20Object%20Reference) (bSelfMoved :type Boolean) (HitLocation :type Vector :default "0, 0, 0") (HitNormal :type Vector :default "0, 0, 0") (NormalImpulse :type Vector :default "0, 0, 0") (Hit :type Hit%20Result%20Structure%20%28by%20ref%29))
  ;[1 1 1] Flying Attack
  (bind _asbp_player (Utilities|Casting|CastToBP_Player Other))
  (Sprite|SetFlipbook (Variables|Default|GetSprite) "/Game/PaperAssets/Boss/Bee_boss/FlipBook/FB_Boss_Attack.FB_Boss_Attack")
  (Game|Damage|ApplyDamage _asbp_player 1.0 0 self)
  (Utilities|FlowControl|Delay 0.2)
  (Sprite|SetFlipbook (Variables|Default|GetSprite) "/Game/PaperAssets/Boss/Bee_boss/FlipBook/FB_Boss_Fly.FB_Boss_Fly")
  (CallFunction|Chase "0, 0, 0" 1.0))

(event EventTick
  (params (DeltaSeconds :type Float%20%28single-precision%29))
  ;[1 1 1] HealthUI
  (if (not (Variables|Default|GetisDead))
    (Progress|SetPercent (Variables|/Game/PaperAssets/Boss/Bee_boss/Boss_BP/Bee_Boss_RF/UI/WB_BuzzLord_Health.WB_BuzzLord_Health_C|GetHealthBar (Variables|Default|GetBuzzLordHealthUI)) (/ (Variables|Default|GetBuzzLordHealth) (Variables|Default|GetMax_BuzzLord_Health)))))

(event Game|Damage|EventAnyDamage
  (params (Damage :type Float%20%28single-precision%29) (DamageType :type Damage%20Type%20Object%20Reference) (InstigatedBy :type Controller%20Object%20Reference) (DamageCauser :type Actor%20Object%20Reference))
  ;[1 1 1] Boss enemy Health
  (if (> (- (.x (Transformation|GetActorLocation DamageCauser)) (.x (Transformation|GetActorLocation self))) 0.0)
    (Character|LaunchCharacter "-1200.000000,0.000000,150.000000" false false)
    (else
      (Character|LaunchCharacter "1200.000000,0.000000,150.000000" false false)))
  (Utilities|FlowControl|Delay 0.1)
  (Sprite|SetFlipbook (Variables|Default|GetSprite) "/Game/PaperAssets/Boss/Bee_boss/FlipBook/FB_Boss_Hit.FB_Boss_Hit")
  (Utilities|FlowControl|Delay 0.2)
  (Sprite|SetFlipbook (Variables|Default|GetSprite) "/Game/PaperAssets/Boss/Bee_boss/FlipBook/FB_Boss_Fly.FB_Boss_Fly")
  (Variables|Default|SetBuzzLordHealth (- (Variables|Default|GetBuzzLordHealth) Damage))
  (if (== (Variables|Default|GetBuzzLordHealth) 0.0)
    (Variables|Default|SetisDead true)
    (CallFunction|BossDeath)
    (elif (== (Variables|Default|GetBuzzLordHealth) 2e+01)
      (Variables|Default|SetIsPhase2 true)
      (CallFunction|MinionSpawnTrigger)
      (else
        (CallFunction|Chase "0, 0, 0" 1.0)))))

(fn ConstructionScript)

(fn HealthCheck)